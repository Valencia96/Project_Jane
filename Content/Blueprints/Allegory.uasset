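; Allegory is an enemy that chases pawns it sees and is repelled by the player's flashlight.
; On each sighting, it moves toward the seen pawn unless the last overlapped component is named PlayerRadius, the player's safe zone.
; If the light is on and touching it, EnemyRepulsion turns it around and teleports it to a fixed offset from Jane.
; The light-contact flag refreshes after that decision, so each sighting uses the previous overlap result.
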(event `self.PawnSensing.OnSeePawn`
  (params (Pawn :type "Pawn Object Reference"))
  (bind _flashlight_ref (`self.Flashlight_ref`))
  (`/Engine/EditorBlueprintResources/StandardMacros.IsValid` _flashlight_ref
    (:`Is Valid`
      (`|ExecutionSequence`
        (:`then_0`
          (bind _lightstate (`/Game/SpotLight2_Blueprint.IsLightOn` _flashlight_ref))
          (if (and _lightstate (stale _touching_))
            (`self.Enemy Repulsion`)
            (else
              (bind _returnvalue (`KismetStringLibrary.EqualEqual_StrStr` (`KismetSystemLibrary.GetDisplayName` (stale `self.CapsuleComponent.OnComponentBeginOverlap` OtherComp)) "PlayerRadius"))
              ;[0.4286 0 1] If not colliding with flashlight "vision"
              (if (not _returnvalue)
                (`|AIMoveTo` self (0.0 0.0 0.0) Pawn 5.0 _returnvalue)))))
        (:`then_1`
          (bind _touching_ (`self.isTouchingFLCapsule` _flashlight_ref)))))
    (:`Is Not Valid`
      (bind _asspot_light_2_blueprint (cast `/Game/SpotLight2_Blueprint` _))
      (set `self.Flashlight_ref` _asspot_light_2_blueprint))))

(event `self.CapsuleComponent.OnComponentBeginOverlap`
  (params (OverlappedComponent :type "PrimitiveComponent Object Reference") (OtherActor :type "Actor Object Reference") (OtherComp :type "PrimitiveComponent Object Reference") (OtherBodyIndex :type Integer) (bFromSweep :type Boolean) (SweepResult :type "HitResult Structure (by ref)"))
  ;[0.4286 3.323 8.636e+15 0.3797] Checking if Enemy is colliding with the Player's "safe zone".
)

(fn `Enemy Repulsion`
  ;[1 1 1] Rotate 180 Degrees
  (`self.K2_SetActorRotation` (`KismetMathLibrary.MakeRotator` 0.0 0.0 (+ (.yaw (`self.K2_GetActorRotation`)) 180.0)))
  (`self.K2_SetActorLocation` (`KismetMathLibrary.MakeVector` (+ (.x (`self.K2_GetActorLocation` (`self.JaneReference`))) 200.0) (+ (.y (`self.K2_GetActorLocation` (`self.JaneReference`))) -200.0)))
  (return))

(fn `isTouchingFLCapsule`
  (params (Target :type "/Game/SpotLight2_Blueprint Object Reference"))
  (returns (`Touching?` :type Boolean))
  (bind _lightcollision (`/Game/SpotLight2_Blueprint.LightCollision` Target)
    (:`then`
      (bind _outcomponents (`KismetSystemLibrary.ComponentOverlapComponents` (`self.CapsuleComponent`) (`KismetMathLibrary.MakeTransform` (0.0 0.0 0.0)) (`|MakeArray` "ObjectTypeQuery4" :!type "EObjectTypeQuery Enum")))
      (bind _returnvalue (`KismetArrayLibrary.Array_Contains` _outcomponents _lightcollision))
      (if _returnvalue
        (return _returnvalue)
        (else
          (`KismetSystemLibrary.PrintString` "NoLight"))))
    (:`else`
      (`KismetSystemLibrary.PrintString` "LightCollisionNotValid"))))

(fn `UserConstructionScript`
  (`parent.UserConstructionScript`))