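; Flashlight Blueprint with a battery timer that sets spotlight visibility and refills, up to a cap, from overlapping Cylinder_Blueprint pickups.
; A short FraudTimer debounces pickups, but also gates the Tick battery and visibility update.
; DecreaseTimer subtracts the battery from DeltaSeconds, flipping its sign rather than steadily draining it.
; Lightshine overlaps match actor names against a list to play a one-shot click at the player.
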(event `self.ReceiveTick`
  (params (DeltaSeconds :type "Float (single-precision)"))
  (bind _fraudtimer (`self.fraudTimer`))
  ;[1 1 1] This is the thing that makes the battery work like a battery (going down)
  (if (> _fraudtimer 0.0)
    (set `self.fraudTimer` (- _fraudtimer DeltaSeconds))
    (`|ExecutionSequence`
      (:`then_0`
        (`self.DecreaseTimer` DeltaSeconds)
        (bind _newparam (`self.IsLightOn`))
        (set `self.lightOn` _newparam))
      (:`then_1`
        (`SceneComponent.SetVisibility` (`self.SpotLightComponent`) (`self.lightOn`) false)))))

(event `self.Box.OnComponentBeginOverlap`
  (params (OverlappedComponent :type "PrimitiveComponent Object Reference") (OtherActor :type "Actor Object Reference") (OtherComp :type "PrimitiveComponent Object Reference") (OtherBodyIndex :type Integer) (bFromSweep :type Boolean) (SweepResult :type "HitResult Structure (by ref)"))
  ;[1 1 1] This is where you add batteries to the flashlight (adds time). includes a fraud timer.
  (bind _fraud_ (`self.BatteryFraudCheck`))
  (if (not _fraud_)
    (set `self.fraudTimer` 0.25)
    (if (`KismetStringLibrary.EqualEqual_StrStr` (`KismetSystemLibrary.GetDisplayName` OtherActor) "Cylinder_Blueprint")
      (`self.AddBattery` 150.0))))

(event `self.Lightshine.OnComponentBeginOverlap`
  (params (OverlappedComponent :type "PrimitiveComponent Object Reference") (OtherActor :type "Actor Object Reference") (OtherComp :type "PrimitiveComponent Object Reference") (OtherBodyIndex :type Integer) (bFromSweep :type Boolean) (SweepResult :type "HitResult Structure (by ref)"))
  (bind _returnvalue (`KismetSystemLibrary.GetDisplayName` OtherActor))
  ;[1 1 1] When light overlaps valid objects, play sound.
  (`WidgetBlueprintLibrary.DrawTextFormatted` (make `PaintContext`) (`KismetTextLibrary.Conv_StringToText` _returnvalue) (100.0 100.0))
  (for _array_element (`self.arrays`)
    (if (== _returnvalue (`KismetStringLibrary.Conv_ObjectToString` _array_element))
      (`/Engine/EditorBlueprintResources/StandardMacros.DoOnce` false
        (:`Completed`
          (`GameplayStatics.PlaySoundAtLocation` "/Game/VRTemplate/Audio/SFX/Flashlight_click_Cue.Flashlight_click_Cue" (`self.K2_GetActorLocation` (`GameplayStatics.GetPlayerPawn` 0)) (struct) 1.0 1.0 0.0 null null OtherActor))))))

(fn `AddBattery`
  (params (NewBattery :type "Float (double-precision)"))
  (bind _returnvalue (+ NewBattery (`self.batteryTimer`)))
  (if (>= NewBattery 330.0)
    (bind _output_get (set `self.batteryTimer` 330.0))
    (`KismetSystemLibrary.PrintString` (`KismetStringLibrary.Conv_DoubleToString` _output_get))
    (elif (>= _returnvalue 330.0)
      (bind _output_get_2 (set `self.batteryTimer` 330.0))
      (`KismetSystemLibrary.PrintString` (`KismetStringLibrary.Conv_DoubleToString` _output_get_2))
      (else
        (bind _output_get_3 (set `self.batteryTimer` _returnvalue))
        (`KismetSystemLibrary.PrintString` (`KismetStringLibrary.Conv_DoubleToString` _output_get_3))))))

(fn `BatteryFraudCheck`
  (returns (`Fraud?` :type Boolean))
  (if (> (`self.fraudTimer`) 0.0)
    (return true)
    (else
      (return false))))

(fn `DecreaseTimer`
  (params (`Delta seconds` :type "Float (double-precision)"))
  (if (`self.lightOn`)
    (set `self.batteryTimer` (- `Delta seconds` (`self.batteryTimer`)))))

(fn `IsLightOn`
  (returns (NewParam :type Boolean))
  (if (> (`KismetMathLibrary.Abs` (`self.batteryTimer`)) 0.0)
    (return true)
    (else
      (return false))))

(fn `UserConstructionScript`)