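; Flashlight Blueprint with a battery timer that controls spotlight visibility on Tick.
; Overlapping an actor named Cylinder_Blueprint with the Box adds battery time up to a cap.
; DecreaseTimer subtracts the timer from DeltaSeconds, reversing the intended countdown, so a charged battery drops below zero within a tick.
; A FraudTimer meant to debounce pickups never counts down while positive, so it blocks overlaps after the first.
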(event `self.ReceiveTick`
  (params (DeltaSeconds :type "Float (single-precision)"))
  ;[1 1 1] This is the thing that makes the battery work like a battery (going down)
  (`|ExecutionSequence`
    (:`then_0`
      (`self.DecreaseTimer` DeltaSeconds)
      (bind _newparam (`self.IsLightOn`))
      (set `self.lightOn` _newparam))
    (:`then_1`
      (`SceneComponent.SetVisibility` (`self.SpotLightComponent`) (`self.lightOn`) false))))

(event `self.Box.OnComponentBeginOverlap`
  (params (OverlappedComponent :type "PrimitiveComponent Object Reference") (OtherActor :type "Actor Object Reference") (OtherComp :type "PrimitiveComponent Object Reference") (OtherBodyIndex :type Integer) (bFromSweep :type Boolean) (SweepResult :type "HitResult Structure (by ref)"))
  ;[1 1 1] This is where you add batteries to the flashlight (adds time). includes a fraud timer to make sure that the
  (bind _fraud_ (`self.BatteryFraudCheck` (stale `self.ReceiveTick` DeltaSeconds)))
  (if (not _fraud_)
    (set `self.fraudTimer` 0.25)
    (if (`KismetStringLibrary.EqualEqual_StrStr` (`KismetSystemLibrary.GetDisplayName` OtherActor) "Cylinder_Blueprint")
      (`self.AddBattery` 150.0))))

(fn `AddBattery`
  (params (NewBattery :type "Float (double-precision)"))
  (bind _returnvalue (+ NewBattery (`self.batteryTimer`)))
  (if (>= NewBattery 330.0)
    (bind _output_get (set `self.batteryTimer` 330.0))
    (`KismetSystemLibrary.PrintString` (`KismetStringLibrary.Conv_DoubleToString` _output_get))
    (elif (>= _returnvalue 330.0)
      (bind _output_get_2 (set `self.batteryTimer` 330.0))
      (`KismetSystemLibrary.PrintString` (`KismetStringLibrary.Conv_DoubleToString` _output_get_2))
      (else
        (bind _output_get_3 (set `self.batteryTimer` _returnvalue))
        (`KismetSystemLibrary.PrintString` (`KismetStringLibrary.Conv_DoubleToString` _output_get_3))))))

(fn `BatteryFraudCheck`
  (params (`Delta Seconds` :type "Float (double-precision)"))
  (returns (`Fraud?` :type Boolean))
  (bind _fraudtimer (`self.fraudTimer`))
  (if (> _fraudtimer 0.0)
    (return true)
    (else
      (set `self.fraudTimer` (- `Delta Seconds` _fraudtimer))
      (return false))))

(fn `DecreaseTimer`
  (params (`Delta seconds` :type "Float (double-precision)"))
  (if (`self.lightOn`)
    (set `self.batteryTimer` (- `Delta seconds` (`self.batteryTimer`)))))

(fn `IsLightOn`
  (returns (NewParam :type Boolean))
  (if (> (`self.batteryTimer`) 0.0)
    (return true)
    (else
      (return false))))

(fn `UserConstructionScript`)